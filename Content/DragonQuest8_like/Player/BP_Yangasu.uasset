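; Player-side Blueprint for the character Yangasu in a Dragon Quest VIII-like battle.
; BeginPlay disables input and calls SearchRecord with the character's ID.
; The Damaged event plays an enemy attack cue, then a physical damage cue, spaced by fixed delays instead of animation callbacks.
; It then sets BattleGameModeBase's state to AnimationFinished, signaling the end of the hit sequence, and prints a debug message.
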(event `self.Damaged`
  (`GameplayStatics.PlaySound2D` "/Game/DragonQuest8_like/Scenes/Battle/SE/Enemy_Attack_Cue.Enemy_Attack_Cue" 1.0 1.0 0.0 null null)
  (`KismetSystemLibrary.Delay` 0.5)
  (`GameplayStatics.PlaySound2D` "/Game/DragonQuest8_like/Scenes/Battle/SE/Damage_Physics_Cue.Damage_Physics_Cue" 1.0 1.0 0.0 null null)
  (`KismetSystemLibrary.Delay` 0.7)
  (bind _asbattle_game_mode_base (cast `BattleGameModeBase` (`GameplayStatics.GetGameMode`)))
  (`BattleGameModeBase.setState` _asbattle_game_mode_base "AnimationFinished")
  (`KismetSystemLibrary.PrintString` "finish"))

(event `self.ReceiveBeginPlay`
  (`self.DisableInput` null)
  (`self.searchRecord` (`self.ID`)))

(fn `UserConstructionScript`)