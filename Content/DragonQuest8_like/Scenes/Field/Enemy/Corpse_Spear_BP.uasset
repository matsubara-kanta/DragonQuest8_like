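; Field enemy, a spear-carrying corpse, that triggers a battle when it hits the player character.
; On hit it destroys itself, saves its enemy ID and the player's position to DQ8GameInstance, then opens the Battle level.
; Each tick it reads the run-direction enum from Corpse_AnimBP and applies a fixed world-axis offset without sweep, so animation state drives movement and speed depends on frame rate.
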(event `self.ReceiveHit`
  (params (MyComp :type "PrimitiveComponent Object Reference") (Other :type "Actor Object Reference") (OtherComp :type "PrimitiveComponent Object Reference") (bSelfMoved :type Boolean) (HitLocation :type "Vector Structure") (HitNormal :type "Vector Structure") (NormalImpulse :type "Vector Structure") (Hit :type "HitResult Structure (by ref)"))
  (cast `/Game/DragonQuest8_like/MyDragonQuest8_likeCharacter` Other)
  (`self.K2_DestroyActor`)
  (bind _asdq8game_instance (cast `DQ8GameInstance` (`GameplayStatics.GetGameInstance`)))
  (set `DQ8GameInstance.enemy_id` (`self.ID`) _asdq8game_instance)
  (set `DQ8GameInstance.player_pos` (`self.K2_GetActorLocation` (`GameplayStatics.GetPlayerPawn` 0)) _asdq8game_instance)
  (`GameplayStatics.OpenLevel` "Battle"))

(event `self.ReceiveTick`
  (params (DeltaSeconds :type "Float (single-precision)"))
  (bind _ascorpse_anim_bp (cast `/Game/DragonQuest8_like/Scenes/Field/Enemy/Corpse_AnimBP` (`SkeletalMeshComponent.GetAnimInstance` (`self.Mesh`))))
  (switch `/Game/DragonQuest8_like/Scenes/Field/Enemy/EnemyEnum` (`/Game/DragonQuest8_like/Scenes/Field/Enemy/Corpse_AnimBP.enum` _ascorpse_anim_bp)
    (:`NewEnumerator1`
      (set `self.Offset` (5.0 0.0 0.0)))
    (:`NewEnumerator2`
      (set `self.Offset` (0.0 -5.0 0.0)))
    (:`NewEnumerator3`
      (set `self.Offset` (0.0 5.0 0.0)))
    (:`NewEnumerator4`
      (set `self.Offset` (-5.0 0.0 0.0))))
  (`self.K2_SetActorLocation` (+ (`self.Offset`) (`self.K2_GetActorLocation`))))

(fn `UserConstructionScript`)