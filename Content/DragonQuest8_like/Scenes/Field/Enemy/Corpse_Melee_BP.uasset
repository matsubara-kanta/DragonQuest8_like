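; Field enemy Blueprint for a melee corpse that starts a battle when the player touches it.
; On a mesh hit with the third-person character, it stores enemy ID and player position in DQ8GameInstance, destroys itself and opens the Battle level.
; Each tick it reads the run-direction enum from Corpse_AnimBP and moves a fixed world-axis step without sweep or delta-time scaling.
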(event `self.MeleeMesh.OnComponentHit`
  (params (HitComponent :type "PrimitiveComponent Object Reference") (OtherActor :type "Actor Object Reference") (OtherComp :type "PrimitiveComponent Object Reference") (NormalImpulse :type "Vector Structure") (Hit :type "HitResult Structure (by ref)"))
  (cast `/Game/ThirdPerson/Blueprints/BP_ThirdPersonCharacter` OtherActor)
  (bind _asdq8game_instance (cast `DQ8GameInstance` (`GameplayStatics.GetGameInstance`)))
  (bind _output_get (set `self.ID` 0))
  (set `DQ8GameInstance.enemy_id` _output_get _asdq8game_instance)
  (set `DQ8GameInstance.player_pos` (`self.K2_GetActorLocation` (`GameplayStatics.GetPlayerPawn` 0)) _asdq8game_instance)
  (`self.K2_DestroyActor`)
  (`GameplayStatics.OpenLevel` "Battle"))

(event `self.ReceiveTick`
  (params (DeltaSeconds :type "Float (single-precision)"))
  (bind _ascorpse_anim_bp (cast `/Game/DragonQuest8_like/Scenes/Field/Enemy/Corpse_AnimBP` (`SkeletalMeshComponent.GetAnimInstance` (`self.MeleeMesh`))))
  (switch `/Game/DragonQuest8_like/Scenes/Field/Enemy/EnemyEnum` (`/Game/DragonQuest8_like/Scenes/Field/Enemy/Corpse_AnimBP.enum` _ascorpse_anim_bp)
    (:`NewEnumerator1`
      (set `self.Offset` (5.0 0.0 0.0)))
    (:`NewEnumerator2`
      (set `self.Offset` (0.0 -5.0 0.0)))
    (:`NewEnumerator3`
      (set `self.Offset` (0.0 5.0 0.0)))
    (:`NewEnumerator4`
      (set `self.Offset` (-5.0 0.0 0.0))))
  (`self.K2_SetActorLocation` (+ (`self.Offset`) (`self.K2_GetActorLocation`))))

(fn `UserConstructionScript`)