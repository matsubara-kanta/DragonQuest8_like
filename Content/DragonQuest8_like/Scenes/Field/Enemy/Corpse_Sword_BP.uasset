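; Sword corpse enemy that starts a battle when the player touches it in the field and also acts as the combatant in battle.
; On player hit, it destroys itself, stores its ID and the player position in the GameInstance, then opens the Battle level.
; When the level name matches, it swaps to the battle AnimBP and looks up its record.
; Damage copies HP to that AnimBP; death triggers delayed destruction.
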(event `self.AnimNotify_Dead`
  (`KismetSystemLibrary.Delay` 1.0)
  (`self.K2_DestroyActor`))

(event `self.Dead`
  (`self.AnimNotify_Dead`))

(event `self.Damaged`
  (bind _enemy_record_hp (break `EnemyDataAssetRecord` (`self.enemy_record`)))
  (bind _ascorpse_batlle_anim_bp (cast `/Game/DragonQuest8_like/Scenes/Field/Enemy/Anim_BP/Corpse_Batlle_AnimBP` (`SkeletalMeshComponent.GetAnimInstance` (`self.Mesh`))))
  (set `/Game/DragonQuest8_like/Scenes/Field/Enemy/Anim_BP/Corpse_Batlle_AnimBP.HP` _enemy_record_hp _ascorpse_batlle_anim_bp))

(event `self.ReceiveBeginPlay`
  (`PrimitiveComponent.SetCollisionResponseToAllChannels` (`self.Mesh`) "ECR_Block")
  (bind _returnvalue (`GameplayStatics.GetCurrentLevelName` true))
  (if (`KismetStringLibrary.EqualEqual_StrStr` _returnvalue (`self.LevelName`))
    (`SkeletalMeshComponent.SetAnimInstanceClass` (`self.Mesh`) "/Game/DragonQuest8_like/Scenes/Field/Enemy/Anim_BP/Corpse_Batlle_AnimBP.Corpse_Batlle_AnimBP_C")
    (`self.searchRecord` (`self.ID`))))

(event `self.ReceiveHit`
  (params (MyComp :type "PrimitiveComponent Object Reference") (Other :type "Actor Object Reference") (OtherComp :type "PrimitiveComponent Object Reference") (bSelfMoved :type Boolean) (HitLocation :type "Vector Structure") (HitNormal :type "Vector Structure") (NormalImpulse :type "Vector Structure") (Hit :type "HitResult Structure (by ref)"))
  (cast `/Game/DragonQuest8_like/MyDragonQuest8_likeCharacter` Other)
  (`self.K2_DestroyActor`)
  (bind _asdq8game_instance (cast `DQ8GameInstance` (`GameplayStatics.GetGameInstance`)))
  (set `DQ8GameInstance.enemy_id` (`self.ID`) _asdq8game_instance)
  (set `DQ8GameInstance.player_pos` (`self.K2_GetActorLocation` (`GameplayStatics.GetPlayerPawn` 0)) _asdq8game_instance)
  (`GameplayStatics.OpenLevel` "Battle"))

(event `self.ReceiveTick`
  (params (DeltaSeconds :type "Float (single-precision)")))

(fn `UserConstructionScript`)