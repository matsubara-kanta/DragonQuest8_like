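; Sword-wielding corpse enemy for a Dragon Quest 8-style RPG, used both as a field encounter and as a battle combatant.
; In the field, a forward trace toggles a camera-facing widget on spotting the player; overlap saves enemy ID and player position, rolls the camera, fades out and opens Battle.
; In the designated level it swaps to the battle AnimBP, loads its record and stops AI.
; Timed attack and damage events drive animation, while death updates the GameMode's count and state.
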(event `self.AnimNotify_Dead`
  (`self.SetLifeSpan` 0.7)
  (`KismetSystemLibrary.Delay` 0.7)
  (bind _asbattle_game_mode_base (cast `BattleGameModeBase` (`GameplayStatics.GetGameMode`)))
  (set `BattleGameModeBase.enemy_deadcount` (+ (`BattleGameModeBase.enemy_deadcount` _asbattle_game_mode_base) 1) _asbattle_game_mode_base)
  (`BattleGameModeBase.setState` _asbattle_game_mode_base "AnimationFinished"))

(event `self.Damaged`
  (bind _enemy_record_hp (break `EnemyDataAssetRecord` (`self.enemy_record`)))
  (bind _ascorpse_batlle_anim_bp (cast `/Game/DragonQuest8_like/Enemy/Anim_BP/Corpse_Batlle_AnimBP` (`SkeletalMeshComponent.GetAnimInstance` (`self.Mesh`))))
  (`GameplayStatics.PlaySound2D` "/Game/DragonQuest8_like/Scenes/Battle/SE/Player_Attack_Cue.Player_Attack_Cue" 1.0 1.0 0.0 null null)
  (`KismetSystemLibrary.Delay` 0.5)
  (`GameplayStatics.PlaySound2D` "/Game/DragonQuest8_like/Scenes/Battle/SE/Damage_Physics_Cue.Damage_Physics_Cue" 1.0 1.0 0.0 null null)
  (`KismetSystemLibrary.Delay` 0.6)
  (set `/Game/DragonQuest8_like/Enemy/Anim_BP/Corpse_Batlle_AnimBP.HP` _enemy_record_hp _ascorpse_batlle_anim_bp)
  (`self.AnimNotify_Dead`))

(event `self.ReceiveBeginPlay`
  (`PrimitiveComponent.SetCollisionResponseToAllChannels` (`self.Mesh`) "ECR_Block")
  (bind _returnvalue (`GameplayStatics.GetCurrentLevelName` true))
  (if (`KismetStringLibrary.EqualEqual_StrStr` _returnvalue (`self.LevelName`))
    (`SkeletalMeshComponent.SetAnimInstanceClass` (`self.Mesh`) "/Game/DragonQuest8_like/Enemy/Anim_BP/Corpse_Batlle_AnimBP.Corpse_Batlle_AnimBP_C")
    (`self.searchRecord` (`self.ID`))
    (`BrainComponent.StopLogic` (`AIController.BrainComponent` (`AIBlueprintHelperLibrary.GetAIController` self)) "")))

(event `self.ReceiveActorBeginOverlap`
  (params (OtherActor :type "Actor Object Reference"))
  (cast `/Game/DragonQuest8_like/Player/MyDragonQuest8_likeCharacter` OtherActor)
  (set `self.NewVar` true)
  (`self.DisableInput` (`GameplayStatics.GetPlayerCharacter` 0) (`GameplayStatics.GetPlayerController` 0))
  (bind _asdq8game_instance (cast `DQ8GameInstance` (`GameplayStatics.GetGameInstance`)))
  (set `DQ8GameInstance.enemy_id` (`self.ID`) _asdq8game_instance)
  (set `DQ8GameInstance.player_pos` (`self.K2_GetActorLocation` (`GameplayStatics.GetPlayerPawn` 0)) _asdq8game_instance)
  (bind _returnvalue (`|CreateWidget` "/Game/DragonQuest8_like/Scenes/Field/FadeOut_W.FadeOut_W_C"))
  (`UserWidget.AddToViewport` _returnvalue 0)
  (`BrainComponent.StopLogic` (`AIController.BrainComponent` (`AIBlueprintHelperLibrary.GetAIController` self)) "")
  (`KismetSystemLibrary.Delay` 1.0)
  (`GameplayStatics.OpenLevel` "Battle"))

(event `self.ReceiveTick`
  (params (DeltaSeconds :type "Float (single-precision)"))
  (if (`self.NewVar`)
    (`self.RotateCamera`)
    (else
      (`self.Detection`))))

(event `self.Attack`
  (bind _ascorpse_batlle_anim_bp (cast `/Game/DragonQuest8_like/Enemy/Anim_BP/Corpse_Batlle_AnimBP` (`SkeletalMeshComponent.GetAnimInstance` (`self.Mesh`))))
  (set `/Game/DragonQuest8_like/Enemy/Anim_BP/Corpse_Batlle_AnimBP.is_Attack` true _ascorpse_batlle_anim_bp)
  (`self.AnimNotify_Attack_Finished`))

(event `self.AnimNotify_Attack_Finished`
  (`KismetSystemLibrary.Delay` 1.33)
  (bind _ascorpse_batlle_anim_bp (cast `/Game/DragonQuest8_like/Enemy/Anim_BP/Corpse_Batlle_AnimBP` (`SkeletalMeshComponent.GetAnimInstance` (`self.Mesh`))))
  (set `/Game/DragonQuest8_like/Enemy/Anim_BP/Corpse_Batlle_AnimBP.is_Attack` false _ascorpse_batlle_anim_bp))

(fn `Detection`
  (locals (Distance :type "Float (double-precision)"))
  (bind _widget (`self.Widget`))
  (bind _widget_2 (`self.Widget`))
  (bind (_returnvalue_roll _returnvalue_pitch) (`KismetMathLibrary.BreakRotator` (`SceneComponent.K2_GetComponentRotation` _widget_2)))
  (bind _returnvalue (+ (`self.K2_GetActorLocation`) (0.0 0.0 65.0)))
  (bind (_returnvalue_roll_2 _returnvalue_pitch_2 _returnvalue_yaw) (`KismetMathLibrary.BreakRotator` (`KismetMathLibrary.FindLookAtRotation` (`SceneComponent.K2_GetComponentLocation` _widget_2) (`PlayerCameraManager.GetCameraLocation` (`GameplayStatics.GetPlayerCameraManager` 0)))))
  (`SceneComponent.K2_SetWorldRotation` _widget_2 (`KismetMathLibrary.MakeRotator` _returnvalue_roll _returnvalue_pitch _returnvalue_yaw) false false)
  (bind (_outhit _returnvalue_2) (`KismetSystemLibrary.LineTraceSingle` :`Start` _returnvalue :`End` (+ _returnvalue (* (`self.GetActorForwardVector`) (`local.Distance`))) :`TraceChannel` "TraceTypeQuery1" :`DrawTime` 0.0))
  (if _returnvalue_2
    (if (`self.ActorHasTag` (`.HitActor` (`GameplayStatics.BreakHitResult` _outhit)) "Player")
      (`SceneComponent.SetVisibility` _widget true false))
    (else
      (`SceneComponent.SetVisibility` _widget false false))))

(fn `RotateCamera`
  (locals (NewLocalVar :type "Float (double-precision)" :default -2.0))
  (bind _angle_roll (`KismetMathLibrary.BreakRotator` (`self.angle`)))
  (bind _asmy_dragon_quest_8_like_character (cast `/Game/DragonQuest8_like/Player/MyDragonQuest8_likeCharacter` (`GameplayStatics.GetPlayerCharacter` 0)))
  (bind _output_get (set `self.angle` (`KismetMathLibrary.MakeRotator` (+ (`local.NewLocalVar`) _angle_roll))))
  (`SceneComponent.K2_SetRelativeRotation` (`DragonQuest8_likeCharacter.FollowCamera` _asmy_dragon_quest_8_like_character) _output_get false false))

(fn `UserConstructionScript`)